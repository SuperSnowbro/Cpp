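; BP_MyBattleHUD is a battle HUD Blueprint that highlights actors in front of the player's BP_BattleCharacter with debug boxes.
; BeginPlay caches the player pawn.
; Each Tick loops over FoundActors, uses a dot product against the pawn's forward vector to keep those ahead, and draws world-space boxes around their bounds.
; Nothing in these graphs fills FoundActors.
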(event `self.ReceiveBeginPlay`
  (set `self.Pawn` (cast `/Game/BP_BattleCharacter` (`GameplayStatics.GetPlayerPawn` 0) :!pure true)))

(event `self.ReceiveTick`
  (params (DeltaSeconds :type "Float (single-precision)"))
  (`/Engine/EditorBlueprintResources/StandardMacros.IsValid` (`self.Pawn`)
    (:`Is Valid`
      (for _array_element (`self.FoundActors`)
        (if (> (`KismetMathLibrary.Dot_VectorVector` (- (`self.K2_GetActorLocation` _array_element) (`self.K2_GetActorLocation` (`self.Pawn`))) (`self.GetActorForwardVector` (`self.Pawn`))) 0.0)
          (bind (_origin _boxextent) (`self.GetActorBounds` _array_element false))
          (`KismetSystemLibrary.DrawDebugBox` _origin _boxextent (struct :`R` 1.0 :`B` 0.853683 :`A` 1.0) (struct) 0.0 4.0))))))

(fn `UserConstructionScript`)